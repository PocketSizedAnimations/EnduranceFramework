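; InteractiveObject is a test actor that responds to the begin, end and cancel events of its Interactive member with debug prints.
; Tick animates its TextRender with a frame-time-based yaw spin and a sine-wave vertical bob.
; Interaction begin also starts a timer on the empty Test function and stores the handle; the remaining-time print is unconnected.
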(event OnInteractionBegin(Interactive)
  (params (Actor :type Actor%20Object%20Reference) (User :type Actor%20Object%20Reference))
  (Development|PrintString "OnInteractionBegin()")
  (bind _returnvalue (Utilities|Time|SetTimerbyFunctionName 0 "Test" 1e+01))
  (Variables|Default|SetTestTimer _returnvalue))

(event OnInteractionEnd(Interactive)
  (params (Actor :type Actor%20Object%20Reference) (User :type Actor%20Object%20Reference))
  (Development|PrintString "OnInteractionEnd()"))

(event OnInteractionCanceled(Interactive)
  (params (Actor :type Actor%20Object%20Reference) (User :type Actor%20Object%20Reference))
  (Development|PrintString "OnInteractionCanceled()"))

(event EventBeginPlay)

(event Collision|EventActorBeginOverlap
  (params (OtherActor :type Actor%20Object%20Reference)))

(event EventTick
  (params (DeltaSeconds :type Float%20%28single-precision%29))
  ;[0.1771 1 1] Animation Text
  (Transformation|AddRelativeRotation (Variables|Default|GetTextRender) (Math|Rotator|MakeRotator 0.0 0.0 (Math|Trig|Sin(Radians) (* DeltaSeconds 5e+01))) false false)
  (Transformation|SetRelativeLocation (Variables|Default|GetTextRender) (Math|Vector|MakeVector 0.0 0.0 (* (Math|Trig|Sin(Radians) (* (Utilities|Time|GetGameTimeinSeconds) 2.0)) 8.0)) false false))

(fn ConstructionScript)

(fn Test)