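; Enemy NPC Blueprint that serves as a debug harness for sense, sound and health components.
; Each tick it prints the alert state from its Senses component, and shortly after BeginPlay it emits an environmental disturbance sound through the audio subsystem.
; Damage events from SimpleHealth and heard-sound events from Senses are printed on screen.
; Alert and aggression setters are present but unconnected.
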(event ClientTakeAnyDamage(SimpleHealth)
  (params (DamagedActor :type Actor%20Object%20Reference) (Damage :type Float%20%28single-precision%29) (DamageType :type Damage%20Type%20Object%20Reference) (InstigatedBy :type Controller%20Object%20Reference) (DamageCauser :type Actor%20Object%20Reference))
  (Development|PrintString (Utilities|String|Append "OUCH : " (Utilities|String|ToString(Float) Damage))))

(event OnSoundHeard(Senses)
  (params (SoundLocation :type Vector :default "0, 0, 0") (SoundCategory :type ESoundCategory%20Enum :default "Environmental") (SoundMaker :type Actor%20Object%20Reference) (SoundInstigator :type Controller%20Object%20Reference))
  (Development|PrintString (Utilities|String|Append "OnSoundHeard(): Location(" (Utilities|String|ToString(Vector) SoundLocation) ") Sound Category(" (Utilities|String|EnumtoString SoundCategory) ") Sound Maker(" (Utilities|GetDisplayName SoundMaker) ") SoundInstigator(" (Utilities|GetDisplayName SoundInstigator) ")")))

(event EventBeginPlay
  (Utilities|FlowControl|Delay 3.5)
  (Class|AudioSubsystem|MakeSound (Subsystems|GetAudioSubsystem) "0, 0, 0" "EnvironmentalDisturbance" 0 0))

(event EventTick
  (params (DeltaSeconds :type Float%20%28single-precision%29))
  (Development|PrintString (Utilities|String|EnumtoString (Class|SensesComponent|GetAlertState (Variables|Default|GetSenses))) true false "(R=0.000000,G=0.660000,B=1.000000,A=1.000000)" 2.0 "Aggro"))

(fn ConstructionScript)