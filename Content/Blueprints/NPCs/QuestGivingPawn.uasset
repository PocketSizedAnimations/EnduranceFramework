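; QuestGivingPawn is an NPC pawn that gives the player a fetch quest.
; When the player pawn overlaps its QuestActivationCollision, it casts to PlayerBlueprint and adds FetchQuest through the player's QuestManager, unless the quest is already held.
; A SimpleHealth damage event prints the damage taken as a debug string.
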(event ClientTakeAnyDamage(SimpleHealth)
  (params (DamagedActor :type Actor%20Object%20Reference) (Damage :type Float%20%28single-precision%29) (DamageType :type Damage%20Type%20Object%20Reference) (InstigatedBy :type Controller%20Object%20Reference) (DamageCauser :type Actor%20Object%20Reference))
  (Development|PrintString (Utilities|String|Append "OUCH : " (Utilities|String|ToString(Float) Damage))))

(event OnComponentBeginOverlap(QuestActivationCollision)
  (params (OverlappedComponent :type Primitive%20Component%20Object%20Reference) (OtherActor :type Actor%20Object%20Reference) (OtherComp :type Primitive%20Component%20Object%20Reference) (OtherBodyIndex :type Integer) (bFromSweep :type Boolean) (SweepResult :type Hit%20Result%20Structure%20%28by%20ref%29))
  (bind _returnvalue (Game|Player|GetPlayerPawn 0))
  (if (== OtherActor _returnvalue)
    (bind _asplayer_blueprint (Utilities|Casting|CastToPlayerBlueprint _returnvalue))
    (if (not (.ReturnValue (Class|QuestManagerComponent|HasQuest (Variables|/Game/Blueprints/PlayerBlueprint.PlayerBlueprint_C|GetQuestManager _asplayer_blueprint) "/Game/Blueprints/FetchQuest.FetchQuest")))
      (Class|QuestManagerComponent|AddQuest (Variables|/Game/Blueprints/PlayerBlueprint.PlayerBlueprint_C|GetQuestManager _asplayer_blueprint) "/Game/Blueprints/FetchQuest.FetchQuest"))))

(event Collision|EventActorBeginOverlap
  (params (OtherActor :type Actor%20Object%20Reference)))

(fn ConstructionScript)