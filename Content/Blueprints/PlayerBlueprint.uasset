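; Player character Blueprint that handles movement, camera look, weapon fire, inventory, quest journal and interaction input.
; Manager components do the work: InventoryManager supplies the equipped Weapon and quickslots, QuestManager toggles the journal, and InteractiveManager starts or cancels interactions.
; Tick rotates the Sphere component to match control rotation.
; EquipPrimary equips the third quickslot or fills it from the first inventory item, while denied interactions play a sound and added quests print a placeholder string.
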(event OnInteractionDenied(InteractiveManager)
  (params (Actor :type Actor%20Object%20Reference) (User :type Actor%20Object%20Reference))
  ;[1 0.4922 0.2488] INTERACTION - DENIED
  (Audio|PlaySound2D "/Game/Audio/Deny_Readout_Interface_Cue.Deny_Readout_Interface_Cue" 1.0 1.0 0.0 0 0))

(event OnQuestAdded(QuestManager)
  (params (QuestManager :type Quest%20Manager%20Component%20Object%20Reference) (Quest :type Quest%20Object%20Reference))
  (Development|PrintString "*PELVIC THRUST INTO MATT*"))

(event EventBeginPlay
  ;[1 0 0.07623] BEGIN PLAY
)

(event EventTick
  (params (DeltaSeconds :type Float%20%28single-precision%29))
  (bind _returnvalue (Pawn|GetController))
  ;[1 0 0.07388] TICK
  ;[0.7035 0.427 1] Update Sphere Rotation to match Controller Look
  (if (Utilities|IsValid _returnvalue)
    (Transformation|SetWorldRotation (Variables|Default|GetSphere) (Pawn|GetControlRotation _returnvalue :!class /Script/Engine.Controller) false false)))

(event Input|ActionEvents|InputActionInteract
  (params (Key :type Key%20Structure :default "None"))
  (bind _interactivemanager (Variables|Default|GetInteractiveManager))
  (bind _returnvalue (Class|InteractiveManagerComponent|GetCurrentInteractive _interactivemanager))
  ;[1 0.4922 0.2488] INPUT - Interaction
  (:Pressed
    (Class|InteractiveManagerComponent|Interact _interactivemanager _returnvalue))
  (:Released
    (Class|InteractiveManagerComponent|CancelInteraction _interactivemanager _returnvalue)))

(event Input|ActionEvents|InputActionOpenInventory
  (params (Key :type Key%20Structure :default "None"))
  (bind _returnvalue (Game|GetPlayerController 0))
  (bind _inventorymanager (Variables|Default|GetInventoryManager))
  ;[0.2475 0.7247 1] Inventory
  (:Released
    (if (Class|InventoryManagerComponent|IsInventoryUIOpen _inventorymanager)
      (Class|InventoryManagerComponent|CloseInventoryUI _inventorymanager _returnvalue)
      (else
        (Class|InventoryManagerComponent|OpenInventoryUI _inventorymanager _returnvalue)))))

(event Input|ActionEvents|InputActionBeginFire
  (params (Key :type Key%20Structure :default "None"))
  (:Pressed
    (bind _asweapon (Utilities|Casting|CastToWeapon (Class|InventoryManagerComponent|GetCurrentlyEquippedItem (Variables|Default|GetInventoryManager))))
    (Class|Weapon|BeginFire _asweapon)))

(event Input|ActionEvents|InputActionEndFire
  (params (Key :type Key%20Structure :default "None"))
  (:Released
    (bind _asweapon (Utilities|Casting|CastToWeapon (Class|InventoryManagerComponent|GetCurrentlyEquippedItem (Variables|Default|GetInventoryManager))))
    (Class|Weapon|EndFire _asweapon)))

(event Input|ActionEvents|InputActionEquipPrimary
  (params (Key :type Key%20Structure :default "None"))
  (:Pressed
    (Utilities|IsValid (Class|InventoryManagerComponent|GetQuickslotItem (Variables|Default|GetInventoryManager) "Quickslot3")
      (:Is%20Valid
        (Class|InventoryManagerComponent|EquipQuickslot (Variables|Default|GetInventoryManager) "Quickslot3"))
      (:Is%20Not%20Valid
        (Class|InventoryManagerComponent|AssigntoQuickslot (Variables|Default|GetInventoryManager) (Utilities|Array|Get(acopy) (Class|InventoryManagerComponent|GetInventory (Variables|Default|GetInventoryManager))) "Quickslot3")))))

(event Input|ActionEvents|InputActionOpenJournal
  (params (Key :type Key%20Structure :default "None"))
  (bind _questmanager (Variables|Default|GetQuestManager))
  ;[0.7273 0.1745 1] Journal Open/Close
  (:Pressed
    (if (Class|QuestManagerComponent|IsJournalWidgetOpened (Variables|Default|GetQuestManager))
      (Class|QuestManagerComponent|CloseJournalWidget _questmanager)
      (else
        (Class|QuestManagerComponent|OpenJournalWidget _questmanager)))))

(event Input|AxisEvents|InputAxisMoveForward
  (params (AxisValue :type Float%20%28single-precision%29))
  ;[0.1367 0.8802 1] INPUT - Movement
  (Class|PawnMovementComponent|AddInputVector (Variables|Character|GetCharacterMovement) (* (Transformation|GetActorForwardVector) AxisValue) false))

(event Input|AxisEvents|InputAxisMoveRight
  (params (AxisValue :type Float%20%28single-precision%29))
  ;[0.1367 0.8802 1] INPUT - Movement
  (Class|PawnMovementComponent|AddInputVector (Variables|Character|GetCharacterMovement) (* (Transformation|GetActorRightVector) AxisValue) false))

(event Input|AxisEvents|InputAxisPitchCamera
  (params (AxisValue :type Float%20%28single-precision%29))
  ;[0.1367 0.8802 1] INPUT - Movement
  (Pawn|Input|AddControllerPitchInput AxisValue))

(event Input|AxisEvents|InputAxisRotateCamera
  (params (AxisValue :type Float%20%28single-precision%29))
  ;[0.1367 0.8802 1] INPUT - Movement
  (Pawn|Input|AddControllerYawInput AxisValue))

(fn ConstructionScript)